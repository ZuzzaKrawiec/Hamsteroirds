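; Trampoline actor that launches the hamster upward when it enters the sphere trigger.
; On overlap it overrides the hamster's sphere physics velocity, keeping X, slightly boosting Y, and flipping Z into an amplified upward bounce with a guaranteed minimum launch speed.
; The skeletal mesh then plays a one-shot bounce animation.
; Other actors are ignored.
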(event `self.Sphere.OnComponentBeginOverlap`
  (params (OverlappedComponent :type "PrimitiveComponent Object Reference") (OtherActor :type "Actor Object Reference") (OtherComp :type "PrimitiveComponent Object Reference") (OtherBodyIndex :type Integer) (bFromSweep :type Boolean) (SweepResult :type "HitResult Structure (by ref)"))
  (bind _aszzhamster_actor (cast `ZZHamsterActor` OtherActor))
  (bind (_returnvalue_x _returnvalue_y _returnvalue_z) (`KismetMathLibrary.BreakVector` (`self.GetVelocity` _aszzhamster_actor)))
  (`PrimitiveComponent.SetPhysicsLinearVelocity` (`ZZHamsterActor.SphereComponent` _aszzhamster_actor) (`KismetMathLibrary.MakeVector_NetQuantize` _returnvalue_x (* _returnvalue_y 1.2) (`KismetMathLibrary.FMax` (* (`KismetMathLibrary.Abs` _returnvalue_z) 1.4) 860.0)) false "None")
  (`SkeletalMeshComponent.PlayAnimation` (`self.SkeletalMesh`) "/Game/SkeletalMeshes/Trampoline/SK_Trampoline_Anim.SK_Trampoline_Anim" false))

(fn `UserConstructionScript`)